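; RobotControler is the AI controller for the FppRobot, running the Robot_BT behavior tree on the Robot_BB blackboard from BeginPlay.
; AI perception updates set the CanSeeEnemy key from the sensed state, but only for the actor stored in the Enemy key.
; The live graph never assigns Enemy; unconnected leftover chains hold a player-as-Enemy setup and an older delayed always-shoot and follow-player loop.
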(event OnTargetPerceptionUpdated(AIPerception)
  (params (Actor :type Actor%20Object%20Reference) (Stimulus :type AI%20Stimulus%20Structure))
  ;[1 1 1] 观察的目标已更新事件
  (if (== Actor (AI|Components|Blackboard|GetValueasObject (AI|GetBlackboard 0) (Utilities|Name|MakeLiteralName "Enemy")))
    (AI|Components|Blackboard|SetValueasBool (AI|GetBlackboard 0) (Utilities|Name|MakeLiteralName "CanSeeEnemy") (.bSuccessfullySensed (Utilities|Struct|BreakAIStimulus Stimulus)))))

(event EventBeginPlay
  (Class|AIController|UseBlackboard "/Game/Blueprints/AI/Robot_BB.Robot_BB")
  (AI|RunBehaviorTree "/Game/Blueprints/AI/Robot_BT.Robot_BT"))

(fn ConstructionScript)

(fn GetRobotShooter
  (bind _asfpp_robot (Utilities|Casting|CastToFppRobot (Pawn|GetControlledPawn)))
  (return _asfpp_robot))