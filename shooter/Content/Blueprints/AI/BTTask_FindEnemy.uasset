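; Behavior tree task that finds an enemy for a robot shooter and stores it in the Blackboard's Enemy key.
; A large-radius multi-sphere trace on the Camera channel gathers Shooters, filtered by IsEnemy, with no break after a match.
; With hits but no enemy, it ends any active gunfire.
; It only finishes with success, but never finishes if hits contain no enemy and the gun is idle.
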(event EventReceiveExecute
  (params (OwnerActor :type Actor%20Object%20Reference))
  (bind _asrobot_controler (Utilities|Casting|CastToRobotControler OwnerActor))
  ;[1 1 1] 球体追踪 在一定范围被感知
  (bind (_outhits _returnvalue) (Collision|MultiSphereTraceByChannel (Transformation|GetActorLocation (Default|GetRobotShooter _asrobot_controler)) (+ (Transformation|GetActorLocation (Default|GetRobotShooter _asrobot_controler)) "0, 0,10.000000") 6e+04 "TraceTypeQuery2" false 0 "None"))
  (if _returnvalue
    (Variables|Default|SetisHaveNoEnemy true)
    (for _array_element _outhits
      (bind _asshooter (Utilities|Casting|CastToShooter (.HitActor (Collision|BreakHitResult _array_element))))
      (if (Default|IsEnemy _asshooter (Default|GetRobotShooter _asrobot_controler))
        (Variables|Default|SetisHaveNoEnemy false)
        (Class|BTFunctionLibrary|SetBlackboardValueasObject (Utilities|Struct|MakeBlackboardKeySelector (Utilities|Array|MakeArray 0) "Enemy") _asshooter)
        (AI|BehaviorTree|FinishExecute true)))
    ;[1 1 1] 判断结束后是否还有开火，若有要结束开火
    (if (Variables|Default|GetisHaveNoEnemy)
      (if (Variables|/Game/Blueprints/Gun.Gun_C|GetIsInFire (Default|GetCurrentGun (Default|GetRobotShooter _asrobot_controler)))
        (Default|EndFire (Default|GetCurrentGun (Default|GetRobotShooter _asrobot_controler)))
        ;[1 1 1] 没有找到敌人也要结束
        (AI|BehaviorTree|FinishExecute true :!label _label))
      (else
        (goto _label)))
    (else
      (goto _label))))