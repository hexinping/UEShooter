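; Automatic hitscan rifle that fires on behalf of its GunOwner and damages FppRobot targets.
; StartFire plays the owner's shoot montage, attaches a looping-fire muzzle effect, fires at once and repeats ShootOnce on a timer.
; ShootOnce line-traces from the owner's camera along control rotation, with debug drawing left on.
; EndFire, guarded by IsInFire, stops the montage, effect and timer.
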(event EventShootOnce
  (bind _gunowner (Variables|Default|GetGunOwner))
  (bind _camera (Variables|/Game/Blueprints/FppShooter.FppShooter_C|GetCamera _gunowner))
  (bind _returnvalue (Transformation|GetWorldLocation _camera))
  ;[1 1 1] 射击造成伤害
  (bind (_outhit _returnvalue_2) (Collision|LineTraceByChannel _returnvalue (+ (* (Math|Vector|GetForwardVector (Pawn|GetControlRotation _gunowner :!class /Script/Engine.Pawn)) 1.5e+03) _returnvalue) "TraceTypeQuery1" false 0 "ForDuration" true "(R=1.000000,G=0.000000,B=0.000000,A=1.000000)" "(R=0.000000,G=1.000000,B=0.000000,A=1.000000)" 2.0))
  (if _returnvalue_2
    (bind _asfpp_robot (Utilities|Casting|CastToFppRobot (.HitActor (Collision|BreakHitResult _outhit))))
    (Default|TakeDamage _asfpp_robot 2e+01)))

(event EventStartFire
  ;[1 1 1] 开火
  (Utilities|FlowControl|Sequence
    (:then_0
      (Animation|PlayAnimMontage (Variables|Default|GetGunOwner) "/Game/Blueprints/FpptShoot_montage.FpptShoot_montage" 1.0 "None")
      (bind _returnvalue (Effects|SpawnEmitterAttached "/Game/Assets/Effects/ParticleSystems/Weapons/AssaultRifle/Muzzle/P_AssaultRifle_MF.P_AssaultRifle_MF" (Variables|Default|GetMuzzle) "None"))
      (Variables|Default|SetFire%20Effects _returnvalue))
    (:then_1
      (CallFunction|ShootOnce)
      (Utilities|Time|SetTimerbyFunctionName 0 "ShootOnce" 0.2 true))
    (:then_2
      (Variables|Default|SetIsInFire true))))

(event EventEndFire
  ;[1 1 1] 结束开火
  (if (Variables|Default|GetIsInFire)
    (Utilities|FlowControl|Sequence
      (:then_0
        (Animation|StopAnimMontage (Variables|Default|GetGunOwner) "/Game/Blueprints/FpptShoot_montage.FpptShoot_montage")
        (Components|DestroyComponent (Variables|Default|GetFire%20Effects)))
      (:then_1
        (Utilities|Time|ClearTimerbyFunctionName 0 "ShootOnce"))
      (:then_2
        (Variables|Default|SetIsInFire false)))))

(fn ConstructionScript
  (|CallParentFunction))