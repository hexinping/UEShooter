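; GameUtils is a shared utility Blueprint for UI control, saving and player lookups.
; Paired functions switch player 0 between paused UI-only input with cursor and unpaused game-only input.
; Save helpers load a BaseSaveGame slot, creating a new object if that fails, or write one back.
; Lookups return the FppShooter player and map offset item keys to textures; the text and color helpers are empty stubs.
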(fn ShowUIControl
  (params (UIRefence :type Widget%20Object%20Reference))
  (bind _returnvalue (Game|GetPlayerController 0))
  (Input|SetInputModeUIOnly _returnvalue UIRefence "DoNotLock")
  (Variables|/Script/Engine.PlayerController|SetbShowMouseCursor _returnvalue true)
  (Game|SetGamePaused 0 true))

(fn ResumGameControl
  (bind _returnvalue (Game|GetPlayerController 0))
  (Input|SetInputModeGameOnly _returnvalue)
  (Variables|/Script/Engine.PlayerController|SetbShowMouseCursor _returnvalue false)
  (Game|SetGamePaused 0 false))

(fn SetUITextandColor
  (params (text :type Text%20Object%20Reference) (txt :type String) (isSetColor :type Boolean)))

(fn GetColor
  (params (index :type Integer))
  (return ""))

(fn LoadfromFile
  (params (fileName :type String))
  ;[1 1 1] 读取文件
  (bind _returnvalue (SaveGame|LoadGamefromSlot fileName))
  (bind _asbase_save_game (Utilities|Casting|CastToBaseSaveGame _returnvalue)
    (:then
      (Development|PrintString 0 "读取成功")
      (return _asbase_save_game))
    (:CastFailed
      (bind _returnvalue_2 (SaveGame|CreateSaveGameObject "/Game/Blueprints/Datas/BaseSaveGame.BaseSaveGame_C"))
      (Development|PrintString 0 "创建成功")
      (return _returnvalue_2))))

(fn SavetoFile
  (params (saveObject :type Base%20Save%20Game%20Object%20Reference) (fileName :type String))
  (SaveGame|SaveGametoSlot saveObject fileName)
  (Development|PrintString 0 "保存成功"))

(fn GetPlayerRefence
  (bind _asfpp_shooter (Utilities|Casting|CastToFppShooter (Game|GetPlayerCharacter 0)))
  (return _asfpp_shooter))

(fn GetItemTexture
  (params (key :type Integer))
  (for _index (range 0 6)
    (if (== key (+ _index 10000))
      (return (Utilities|Array|Get(acopy) (LocalVariables|GetTextureArray) _index)))))