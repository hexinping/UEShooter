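; Game mode for a first-person shooter that creates the HUD, spawns robots and tracks kill statistics.
; On play it shows the Fpp_UI widget; SpawnRotbot spawns an AI FppRobot at a given actor's location and assigns its side.
; Two maps count kills and deaths per key, though GetKillNum checks an empty key rather than the one passed.
; It also keeps an incrementing index and can print a name array.
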(event EventBeginPlay
  (bind _returnvalue (UserInterface|CreateWidget "/Game/Blueprints/UI/Fpp_UI.Fpp_UI_C"))
  (UserInterface|Viewport|AddtoViewport _returnvalue 0)
  (Variables|Default|SetFppUI _returnvalue))

(event EventTick
  (params (DeltaSeconds :type Float%20%28single-precision%29)))

(fn ConstructionScript)

(fn SpawnRotbot
  (params (side :type Integer) (nearActor :type Actor%20Object%20Reference))
  (bind _returnvalue (AI|SpawnAIFromClass "/Game/Blueprints/FppRobot.FppRobot_C" 0 (Transformation|GetActorLocation nearActor) "0, 0, 0" false))
  (bind _asfpp_robot (Utilities|Casting|CastToFppRobot _returnvalue))
  (Variables|/Game/Blueprints/Shooter.Shooter_C|SetSide _asfpp_robot side)
  (return))

(fn SetIndex
  (Variables|Default|Setindex (+ (Variables|Default|Getindex) 1)))

(fn GetIndex
  (return (Variables|Default|Getindex)))

(fn UpdateKillMap
  (params (key :type String))
  (bind _killmap (Variables|Default|GetKillMap))
  (if (Utilities|Map|Contains _killmap key)
    (Utilities|Map|Add _killmap key (+ (.Value (Utilities|Map|Find _killmap key)) 1))
    (else
      (Utilities|Map|Add _killmap key 1))))

(fn GetKillNum
  (params (key :type String))
  (bind _killmap (Variables|Default|GetKillMap))
  (if (Utilities|Map|Contains _killmap "")
    (return (.Value (Utilities|Map|Find _killmap key)))
    (else
      (return 0))))

(fn GetKilledNum
  (params (key :type String))
  (bind _killedmap (Variables|Default|GetKilledMap))
  (if (Utilities|Map|Contains _killedmap key)
    (return (.Value (Utilities|Map|Find _killedmap key)))
    (else
      (return 0))))

(fn PrintNameArray
  (for _array_element (Variables|Default|GetNameArray)
    (Development|PrintString (Utilities|String|Append "Name:" _array_element) true true "(R=0.000000,G=0.660000,B=1.000000,A=1.000000)" 1e+01)))

(fn UpdateKilledMap
  (params (key :type String))
  (bind _killedmap (Variables|Default|GetKilledMap))
  (if (Utilities|Map|Contains _killedmap key)
    (Utilities|Map|Add _killedmap key (+ (.Value (Utilities|Map|Find _killedmap key)) 1))
    (else
      (Utilities|Map|Add _killedmap key 1))))