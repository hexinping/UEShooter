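; AI controller for FppRobot enemies that shoot constantly while chasing the player.
; After a short BeginPlay delay, which lets the robot get its gun first, it calls AlwaysShoot on the possessed robot.
; It then loops AIMoveTo toward the player within an acceptance radius, pausing briefly after success or failure.
; A RunBehaviorTree node for Robot_BT is present but unconnected.
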(event EventBeginPlay
  ;[1 1 1] controler的begin事件跟robot的begin事件没有明显的先后顺序，这里让controle的后发生，确保机器人已经有枪
  (Utilities|FlowControl|Delay 0.2)
  (Default|AlwaysShoot (CallFunction|GetRobotShooter))
  (AI|AIMoveTo (Pawn|GetControlledPawn) "0, 0, 0" (Game|GetPlayerCharacter 0) 5e+02 false :!label _label
    (:OnSuccess
      _)
    (:OnFail
      _))
  (Utilities|FlowControl|Delay 1.0)
  (goto _label))

(fn ConstructionScript)

(fn GetRobotShooter
  (bind _asfpp_robot (Utilities|Casting|CastToFppRobot (Pawn|GetControlledPawn)))
  (return _asfpp_robot))