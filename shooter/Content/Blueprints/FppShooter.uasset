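; FppShooter is the first-person player character, handling movement, look, firing and weapon switching.
; It creates a launcher and a rifle on BeginPlay, forwards fire input to the current gun, and cycles guns by hiding and showing them with an equip montage and UI update.
; It supplies aim from camera location and control rotation.
; On death, it pulls the camera back and ragdolls a swapped-in third-person mesh.
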(event Collision|EventActorBeginOverlap
  (params (OtherActor :type Actor%20Object%20Reference)))

(event EventTick
  (params (DeltaSeconds :type Float%20%28single-precision%29)))

(event EventBeginPlay
  (CallFunction|CreateGun "/Game/Blueprints/Launcher.Launcher_C")
  (CallFunction|CreateGun "/Game/Blueprints/Rifle.Rifle_C")
  (Variables|Default|SetCurrentIndex 1)
  (Rendering|SetActorHiddenInGame (CallFunction|GetCurrentGun) false))

(event EventOnDie
  (bind _mesh (Variables|Character|GetMesh))
  (Transformation|AddLocalOffset (Variables|Default|GetCamera) "-400.000000, 0, 0" false false)
  (Class|SkinnedMeshComponent|SetSkeletalMesh _mesh "/Game/Assets/Characters/Models/HeroTPP.HeroTPP" true)
  (Physics|SetSimulatePhysics _mesh true)
  (Collision|SetCollisionEnabled _mesh "QueryAndPhysics"))

(event Input|ActionEvents|InputActionFire
  (params (Key :type Key%20Structure :default "AnyKey"))
  (:Pressed
    (CallFunction|StartFire))
  (:Released
    (CallFunction|EndFire)))

(event Input|ActionEvents|InputActionEquip
  (params (Key :type Key%20Structure :default "AnyKey"))
  (:Pressed
    (CallFunction|SwitchWeapon)
    (Default|CallUpdateHpUI (Variables|/Game/Blueprints/ShootGameMode.ShootGameMode_C|GetFppUI (CallFunction|GetCurrGameMode)) "UpdateBulletNum")))

(event Input|AxisEvents|InputAxisMoveForward
  (params (AxisValue :type Float%20%28single-precision%29))
  ;[1 1 1] 沿着人物正向移动
  (Pawn|Input|AddMovementInput (Math|Rotator|GetRotationXVector (Pawn|GetControlRotation :!class /Script/Engine.Pawn)) AxisValue false))

(event Input|AxisEvents|InputAxisLookUp
  (params (AxisValue :type Float%20%28single-precision%29))
  ;[1 1 1] 上下看
  (Pawn|Input|AddControllerPitchInput AxisValue))

(event Input|AxisEvents|InputAxisMoveRight
  (params (AxisValue :type Float%20%28single-precision%29))
  ;[1 1 1] 沿着人物左右移动
  (Pawn|Input|AddMovementInput (Math|Vector|GetRightVector (Pawn|GetControlRotation :!class /Script/Engine.Pawn)) AxisValue false))

(event Input|AxisEvents|InputAxisTurn
  (params (AxisValue :type Float%20%28single-precision%29))
  ;[1 1 1] 朝向
  (Pawn|Input|AddControllerYawInput AxisValue))

(fn ConstructionScript
  (|CallParentFunction))

(fn StartFire
  (Default|StartFire (CallFunction|GetCurrentGun)))

(fn EndFire
  (Default|EndFire (CallFunction|GetCurrentGun)))

(fn SwitchWeapon
  (bind _gun (CallFunction|GetCurrentGun))
  (Default|EndFire _gun)
  (Rendering|SetActorHiddenInGame _gun true)
  (Variables|Default|SetCurrentIndex (Math|Integer|%(Integer) (+ (Variables|Default|GetCurrentIndex) 1) (Utilities|Array|Length (Variables|Default|GetGuns))))
  (Rendering|SetActorHiddenInGame (CallFunction|GetCurrentGun) false)
  (Animation|PlayAnimMontage "/Game/Blueprints/Animations/FppEquip_Montage.FppEquip_Montage" 1.0 "None"))

(fn GetShootLocation
  (return (Transformation|GetWorldLocation (Variables|Default|GetCamera))))

(fn GetShootDirection
  (return (Math|Vector|GetForwardVector (Pawn|GetControlRotation :!class /Script/Engine.Pawn))))