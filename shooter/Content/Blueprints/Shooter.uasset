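; Shooter is a character Blueprint with health, side-based enemy checks and an inventory of guns.
; CreateGun spawns guns hidden on the right weapon socket, and GetCurrentGun picks one by index; all are destroyed with the shooter.
; TakeDamage triggers Die at zero health, which stops all firing, calls OnDie and detaches the controller after a short timer.
; OnDie and the shoot location and direction getters are stubs, returning nothing or zero vectors.
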(event EventBeginPlay)

(event Collision|EventActorBeginOverlap
  (params (OtherActor :type Actor%20Object%20Reference)))

(event EventTick
  (params (DeltaSeconds :type Float%20%28single-precision%29)))

(event EventDestroyed
  ;[1 1 1] 销毁枪
  (for _array_element (Variables|Default|GetGuns)
    (Actor|DestroyActor _array_element)))

(fn ConstructionScript)

(fn TakeDamage
  (params (damage :type Float%20%28single-precision%29))
  (if (not (CallFunction|IsDead))
    (bind _output_get (Variables|Default|SetHealth (- (Variables|Default|GetHealth) damage)))
    (Development|PrintString (Utilities|String|ToString(Float) _output_get))
    (if (CallFunction|IsDead)
      (CallFunction|Die))))

(fn IsDead
  (return (<= (Variables|Default|GetHealth) 0.0)))

(fn GetShootLocation
  (return "0, 0, 0"))

(fn CreateGun
  (params (GunClass :type Gun%20Class%20Reference))
  (bind _returnvalue (Game|SpawnActorfromClass GunClass (Math|Transform|MakeTransform "0, 0, 0" "0, 0, 0" "1,1,1") "Undefined" 0 0))
  (Utilities|Array|Add (Variables|Default|GetGuns) _returnvalue)
  (Variables|/Game/Blueprints/Gun.Gun_C|SetGunOwner _returnvalue self)
  (Transformation|AttachComponentToComponent _returnvalue (Variables|Character|GetMesh) "b_RightWeaponSocket" "SnapToTarget" "SnapToTarget" "SnapToTarget" true)
  (Rendering|SetActorHiddenInGame _returnvalue true))

(fn GetCurrentGun
  (return (Utilities|Array|Get(acopy) (Variables|Default|GetGuns) (Variables|Default|GetCurrentIndex))))

(fn OnDie)

(fn Die
  (for _array_element (Variables|Default|GetGuns)
    (Default|EndFire _array_element))
  (CallFunction|OnDie)
  (Utilities|Time|SetTimerbyFunctionName 0 "DetachFromControllerPendingDestroy" 0.1))

(fn GetShootDirection
  (return "0, 0, 0"))

(fn IsEnemy
  (params (shoot :type Shooter%20Object%20Reference))
  (return (!= (Variables|Shooter_C|GetSide shoot) (Variables|Default|GetSide))))

(fn IsRobot
  (return (== (Variables|Default|GetSide) 1)))