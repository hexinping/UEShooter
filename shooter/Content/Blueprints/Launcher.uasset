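; Launcher weapon Blueprint, a child of a gun base class, that fires single projectiles for a first-person character.
; StartFire fires only when not reloading, not already firing and enough bullets remain.
; ShootOnce spawns a bullet at the muzzle along the owner's control rotation, decrements ammo, refreshes the UI, plays a montage and holds a short cooldown.
; The reload event calls the parent, then plays the launcher reload montage.
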(event EventStartFire
  ;[1 1 1] 上子弹不能开火
  (if (not (Variables|Default|GetisInReloadBullet))
    (if (not (Variables|Default|GetIsInFire))
      (if (CallFunction|IsHaveEnoughBullet)
        (CallFunction|ShootOnce)))))

(event EventShootOnce
  (bind _gunowner (Variables|Default|GetGunOwner))
  (Variables|Default|SetIsInFire true)
  (Game|SpawnActorfromClass "/Game/Blueprints/Bullet.Bullet_C" (Math|Transform|MakeTransform (Transformation|GetWorldLocation (Variables|Default|GetMuzzle)) (Pawn|GetControlRotation (Variables|Default|GetGunOwner) :!class /Script/Engine.Pawn) "1,1,1") "Undefined" 0 _gunowner 0)
  (Variables|Default|SetCurrentBulletNum (- (Variables|Default|GetCurrentBulletNum) 1))
  (Default|CallUpdateHpUI (Variables|/Game/Blueprints/ShootGameMode.ShootGameMode_C|GetFppUI (Default|GetCurrGameMode _gunowner)) "UpdateBulletNum")
  (Animation|PlayAnimMontage (Variables|Default|GetGunOwner) "/Game/Blueprints/Animations/FppLauncher_Montage.FppLauncher_Montage" 1.0 "None")
  (Utilities|FlowControl|Delay 0.4)
  (Variables|Default|SetIsInFire false))

(event EventPlayerGunReloadAnimatin
  (|CallParentFunction)
  (Animation|PlayAnimMontage (Variables|Default|GetGunOwner) "/Game/Blueprints/Animations/FppShootLauncherReload_montage.FppShootLauncherReload_montage" 1.0 "None"))

(fn ConstructionScript
  (|CallParentFunction))